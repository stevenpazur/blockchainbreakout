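; Game instance for Blockchain Breakout that preloads primary assets at startup and plays music that persists across level transitions.
; Init fires five async primary asset loads, each completion decrementing a printed counter.
; When the counter reaches zero, a short delay precedes the assets-loaded call and the finished flag.
; Init also runs a debug pass over primary asset IDs with an empty loop body.
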(event `Play Music`
  (bind _returnvalue (`GameplayStatics.SpawnSound2D` "/Game/Audio/game_sound.game_sound" 1.0 1.0 0.0 null true))
  (set `self.Music` _returnvalue))

(event `self.ReceiveInit`
  (`|ExecutionSequence`
    (:`then_0`
      ;[1 1 1] Preload Primary Assets
      (`AsyncActionLoadPrimaryAsset.AsyncLoadPrimaryAsset` "UI:W_MainMenu2"
        (:`then`
          (`AsyncActionLoadPrimaryAsset.AsyncLoadPrimaryAsset` "UI:W_Options"
            (:`then`
              (`AsyncActionLoadPrimaryAsset.AsyncLoadPrimaryAsset` "Map:/Game/Maps/MainMenu"
                (:`then`
                  (`AsyncActionLoadPrimaryAsset.AsyncLoadPrimaryAsset` "Map:/Game/Maps/OptionsMenu"
                    (:`then`
                      (`AsyncActionLoadPrimaryAsset.AsyncLoadPrimaryAsset` "Map:/Game/Maps/TetrisGridLevel"
                        (:`Completed`
                          (`self.Decrement Assets To Load`))))
                    (:`Completed`
                      (`self.Decrement Assets To Load`))))
                (:`Completed`
                  (`self.Decrement Assets To Load`))))
            (:`Completed`
              (`self.Decrement Assets To Load`))))
        (:`Completed`
          (`self.Decrement Assets To Load`))))
    (:`then_1`
      (`self.Debug Primary Assets`))))

(event `Decrement Assets To Load`
  (bind _result (`/Engine/EditorBlueprintResources/StandardMacros.DecrementInt` (`self.AssetsToLoad`))
    (:`  `
      (`KismetSystemLibrary.PrintString` (`KismetStringLibrary.Conv_IntToString` _result))
      (if (<= (`self.AssetsToLoad`) 0)
        (`KismetSystemLibrary.Delay` 0.5)
        (`self.AssetsLoaded`)
        (set `self.AssetsFinishedLoading` true)))))

(event `Debug Primary Assets`
  (bind _outprimaryassetidlist (`KismetSystemLibrary.GetPrimaryAssetIdList` "Map"))
  (for _ _outprimaryassetidlist
    _))